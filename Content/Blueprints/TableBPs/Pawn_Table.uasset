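; Pawn for table mode that lets the player click and drag physics objects with the mouse, and exit the mode via Interact unless a minigame is running.
; A cursor trace grabs movable, simulating components with a PhysicsHandle and spawns a BP_TracePlane at the hit's Y.
; Each tick the handle follows the cursor trace, with the held item's query collision disabled.
; Releasing restores collision and destroys the plane.
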(event Input|EnhancedActionEvents|EnhancedInputActionIA_TapClick
  (params (ActionValue :type Boolean) (ElapsedSeconds :type Float%20%28double-precision%29) (TriggeredSeconds :type Float%20%28double-precision%29) (InputAction :type Input%20Action%20Object%20Reference :default "/Game/Blueprints/Character/Input/IA_TapClick.IA_TapClick"))
  (:Started
    (if (Variables|/Game/Blueprints/GM_Base.GM_Base_C|GetTableMode (Variables|Default|GetGame%20Mode))
      ;[1 1 1] AttachItemToHandle
      (bind (_outhit _returnvalue) (CallFunction|LineTraceHit))
      (if _returnvalue
        (Variables|Default|SetInitialHit _outhit)
        (if (== (Variables|/Script/Engine.SceneComponent|GetMobility (.HitComponent (Collision|BreakHitResult (Variables|Default|GetInitialHit)))) (Utilities|Enum|LiteralenumEComponentMobility "Movable"))
          (Variables|Default|SetGrabbedComponent (.HitComponent (Collision|BreakHitResult (Variables|Default|GetInitialHit))))
          (if (Physics|IsSimulatingPhysics (Variables|Default|GetGrabbedComponent) "None")
            (Class|PhysicsHandleComponent|GrabComponentatLocation (Variables|Default|GetPhysicsHandle) (Variables|Default|GetGrabbedComponent) "None" (.Location (Collision|BreakHitResult (Variables|Default|GetInitialHit))))
            (Variables|Default|SetItemGrabbed true)
            (Collision|SetCollisionEnabled (Variables|Default|GetGrabbedComponent) "PhysicsOnly")
            (bind _returnvalue_2 (CallFunction|CreateTracePlane))
            (Variables|Default|SetTracePlane _returnvalue_2))))))
  (:Completed
    ;[0.513 0.1173 0.1122] DetachItemFromHandle
    (Utilities|IsValid (Variables|Default|GetGrabbedComponent)
      (:Is%20Valid
        (Collision|SetCollisionEnabled (Variables|Default|GetGrabbedComponent) "QueryAndPhysics"))
      (:Is%20Not%20Valid
        _))
    (Variables|Default|SetGrabbedComponent 0)
    (Variables|Default|SetItemGrabbed false)
    (Physics|Components|PhysicsHandle|ReleaseComponent (Variables|Default|GetPhysicsHandle))
    (Utilities|IsValid (Variables|Default|GetTracePlane)
      (:Is%20Valid
        (Actor|DestroyActor (Variables|Default|GetTracePlane))))))

(event Input|EnhancedActionEvents|EnhancedInputActionIA_Interact
  (params (ActionValue :type Boolean) (ElapsedSeconds :type Float%20%28double-precision%29) (TriggeredSeconds :type Float%20%28double-precision%29) (InputAction :type Input%20Action%20Object%20Reference :default "/Game/Blueprints/Character/Input/IA_Interact.IA_Interact"))
  (bind _game_mode (Variables|Default|GetGame%20Mode))
  (:Started
    (if (not (Variables|/Game/Widgets/Sub_widget/W_Minigame.W_Minigame_C|GetMiniGameOngoing (Variables|/Game/Widgets/W_MainWidget.W_MainWidget_C|GetMiniGame (Variables|/Game/Blueprints/GM_Base.GM_Base_C|GetMainWidget _game_mode))))
      (Default|ExitTableMode _game_mode))))

(event EventBeginPlay
  (bind _asgm_base (Utilities|Casting|CastToGM_Base (Game|GetGameMode)))
  (Variables|Default|SetGame%20Mode _asgm_base))

(event EventTick
  (params (DeltaSeconds :type Float%20%28single-precision%29))
  (Utilities|FlowControl|Sequence
    (:then_0
      ;[0.1019 0.4322 1] MoveObject
      (if (Variables|Default|GetItemGrabbed)
        (Utilities|IsValid (Variables|Default|GetGrabbedComponent)
          (:Is%20Valid
            (bind _outhit (CallFunction|LineTraceHit))
            (Physics|Components|PhysicsHandle|SetTargetLocation (Variables|Default|GetPhysicsHandle) (.Location (Collision|BreakHitResult _outhit)))))))))

(fn ConstructionScript)

(fn LineTraceHit
  (bind _returnvalue (Game|GetPlayerController 0))
  (bind (_worldlocation _worlddirection) (Game|Player|ConvertMouseLocationToWorldSpace _returnvalue))
  (bind (_outhit _returnvalue_2) (Collision|LineTraceByChannel _worldlocation (+ _worldlocation (* _worlddirection 3e+03)) "TraceTypeQuery1" false 0 "None" true "(R=1.000000,G=0.000000,B=0.000000,A=1.000000)" "(R=0.000000,G=1.000000,B=0.000000,A=1.000000)" 2e+01))
  (return _outhit _returnvalue_2))

(fn CreateTracePlane
  (bind _returnvalue (Game|SpawnActorfromClass "/Game/Blueprints/TableBPs/BP_TracePlane.BP_TracePlane_C" (Math|Transform|MakeTransform (Math|Vector|MakeVector 0.0 (.Y (Math|Vector|BreakVector (.Location (Collision|BreakHitResult (Variables|Default|GetInitialHit))))) 0.0) "0, 0, 0" "1.000000,1.000000,1.000000") "Undefined" "MultiplyWithRoot" 0 0))
  (return _returnvalue))