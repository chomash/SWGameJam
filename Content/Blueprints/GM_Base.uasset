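; Game mode for a timed cauldron crafting game where guests order random CookBook recipes, scoring points for correct deliveries.
; Each order spawns a guest via BP_GuestSpawner and updates the order widget; a matching BP_Delliver item or a timeout triggers the next.
; Tick polls the guest and whole-game deadlines, pausing with a finish screen at game end.
; Also switches possession, cursor and input context between map character and table pawn.
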(event Custom|OpenTableMode
  (bind _playercontroller (Variables|Default|GetPlayerController))
  ;[1 1 1] TableModeChange
  (Variables|Default|SetTableMode true)
  (bind _returnvalue (Actor|GetActorOfClass "/Game/Blueprints/TableBPs/Pawn_Table.Pawn_Table_C"))
  (Utilities|IsValid _returnvalue
    (:Is%20Valid
      (Pawn|Possess (Variables|Default|GetPlayerController) _returnvalue)
      (Variables|/Script/Engine.PlayerController|SetbShowMouseCursor _playercontroller true)
      (Input|AddMappingContext (PlayerController|LocalPlayerSubsystems|GetEnhancedInputLocalPlayerSubsystem _playercontroller) "/Game/Blueprints/Character/Input/IMC_Table.IMC_Table" 0 "(bIgnoreAllPressedKeysUntilRelease=True,bForceImmediately=False,bNotifyUserSettings=False)")
      (Default|OpenTable (Variables|ActorRef|GetClaudronActor)))))

(event Custom|ExitTableMode
  (bind _playercontroller (Variables|Default|GetPlayerController))
  ;[1 1 1] TableModeChange
  (Variables|Default|SetTableMode false)
  (bind _returnvalue (Actor|GetActorOfClass "/Game/Blueprints/Character/BP_PlayerMapCharacter.BP_PlayerMapCharacter_C"))
  (Utilities|IsValid _returnvalue
    (:Is%20Valid
      (Pawn|Possess (Variables|Default|GetPlayerController) _returnvalue)
      (Variables|/Script/Engine.PlayerController|SetbShowMouseCursor _playercontroller false)
      (Input|AddMappingContext (PlayerController|LocalPlayerSubsystems|GetEnhancedInputLocalPlayerSubsystem _playercontroller) "/Game/Blueprints/Character/Input/IMC_Map.IMC_Map" 0 "(bIgnoreAllPressedKeysUntilRelease=True,bForceImmediately=False,bNotifyUserSettings=False)")
      (Variables|/Game/Widgets/Sub_widget/W_Minigame.W_Minigame_C|SetCanBePlayed (Variables|/Game/Widgets/W_MainWidget.W_MainWidget_C|GetMiniGame (Variables|Default|GetMainWidget)) false))))

(event Custom|SpawnNewClient
  ;[1 1 1] SpawnNewClient
  (bind _outrownames (DataTable|GetDataTableRowNames "/Game/Recipes/CookBook.CookBook"))
  (bind _returnvalue (Utilities|GetDataTableRow "/Game/Recipes/CookBook.CookBook" (Utilities|Array|Get(acopy) _outrownames (Math|Random|RandomInteger (Utilities|Array|Length _outrownames))))
    (:then
      (Variables|Default|SetRecipeToCraft _returnvalue)
      (bind _newguest (Default|GestSpawning (Variables|ActorRef|GetGuestSpawner)))
      (Variables|ActorRef|SetActiveGuest _newguest)
      (Variables|Timers|SetClientTargetTime (+ (Variables|Timers|GetWaitTime) (Utilities|Time|GetGameTimeinSeconds)))
      (Variables|Timers|SetLookAtClientTime true)
      (CallFunction|UpdateOrder))))

(event Custom|CheckIfRecipeMatch
  ;[1 1 1] CheckRecipe
  (bind _returnvalue (Actor|GetActorOfClass "/Game/Blueprints/Furnitures/BP_Delliver.BP_Delliver_C"))
  (Utilities|IsValid (Variables|/Game/Blueprints/Furnitures/BP_Delliver.BP_Delliver_C|GetHeldItem _returnvalue)
    (:Is%20Valid
      (if (Utilities|Enum|Equal(Enum) (.name (Variables|/Game/Blueprints/PickUps/Childs/BP_MapItem_Potion.BP_MapItem_Potion_C|GetReadyRecipe (Variables|/Game/Blueprints/Furnitures/BP_Delliver.BP_Delliver_C|GetHeldItem _returnvalue))) (.Name (Utilities|Struct|BreakRecipe (Variables|Default|GetRecipeToCraft))))
        (Actor|DestroyActor (Variables|/Game/Blueprints/Furnitures/BP_Delliver.BP_Delliver_C|GetHeldItem _returnvalue))
        (Utilities|FlowControl|Delay 0.5)
        (Default|GuestExit (Variables|ActorRef|GetActiveGuest))
        (Variables|Points|SetPointCounter (+ (Variables|Points|GetPointCounter) (Variables|Points|GetPositivePoint)))
        (CallFunction|SpawnNewClient)))))

(event Custom|ResetState
  (Variables|Points|SetPointCounter 0)
  (Variables|Timers|SetWholeGameTargetTime (+ (Utilities|Time|GetGameTimeinSeconds) (Variables|Timers|GetWholeGameLength)))
  (Variables|Timers|SetLookAtTime true)
  (Variables|Default|SetCanBePaused true))

(event Custom|GameEnd
  (Game|SetGamePaused true)
  (bind _returnvalue (UserInterface|CreateWidget "/Game/Widgets/W_GameFinished.W_GameFinished_C"))
  (UserInterface|Viewport|AddtoViewport _returnvalue 0))

(event Custom|UpdateOrder
  (CallFunction|UpdateOrderWidget))

(event EventBeginPlay
  (bind _aspc_base (Utilities|Casting|CastToPC_Base (Game|GetPlayerController 0)))
  (Variables|Default|SetPlayerController _aspc_base)
  (bind _returnvalue (Actor|GetActorOfClass "/Game/Blueprints/TableBPs/Claudron.Claudron_C"))
  (Variables|ActorRef|SetClaudronActor _returnvalue)
  (bind _returnvalue_2 (UserInterface|CreateWidget "/Game/Widgets/W_MainWidget.W_MainWidget_C"))
  (Variables|Default|SetMainWidget _returnvalue_2)
  (UserInterface|Viewport|AddtoViewport _returnvalue_2 0)
  (bind _returnvalue_3 (Actor|GetActorOfClass "/Game/Blueprints/Guests/BP_GuestSpawner.BP_GuestSpawner_C"))
  (Variables|ActorRef|SetGuestSpawner _returnvalue_3)
  (CallFunction|SpawnNewClient))

(event EventTick
  (params (DeltaSeconds :type Float%20%28single-precision%29))
  (if (Variables|Timers|GetLookAtTime)
    (Utilities|FlowControl|Sequence
      (:then_0
        (if (>= (Utilities|Time|GetGameTimeinSeconds) (Variables|Timers|GetWholeGameTargetTime))
          (Variables|Timers|SetLookAtTime false)
          (CallFunction|GameEnd)))
      (:then_1
        (if (Variables|Timers|GetLookAtClientTime)
          (if (>= (Utilities|Time|GetGameTimeinSeconds) (Variables|Timers|GetClientTargetTime))
            (Variables|Timers|SetLookAtClientTime false)
            (Default|GuestExit (Variables|ActorRef|GetActiveGuest))
            (Variables|Points|SetPointCounter (Math|Integer|Clamp(Integer) (- (Variables|Points|GetPointCounter) (Variables|Points|GetNegativePoint)) 0 99999))
            (CallFunction|SpawnNewClient)))))))

(fn ConstructionScript)

(fn UpdateOrderWidget
  (bind _randomizedcolor (Variables|Default|GetRandomizedColor))
  (bind _recipetocraft (Variables|Default|GetRecipeToCraft))
  (bind _mainwidget (Variables|Default|GetMainWidget))
  (bind (_name _item00 _item01 _item02 _item03 _recipeimage) (Utilities|Struct|BreakRecipe _recipetocraft))
  (bind _w_order (Variables|/Game/Widgets/W_MainWidget.W_MainWidget_C|GetW_Order _mainwidget))
  (bind _w_orderrecpe (Variables|/Game/Widgets/Sub_widget/W_Order.W_Order_C|GetW_OrderRecpe _w_order))
  (Variables|/Script/UMG.Image|SetColorAndOpacity (Variables|/Game/Widgets/Sub_widget/W_Order.W_Order_C|GetGuestPortrait _w_order) (Utilities|Array|Get(acopy) _randomizedcolor (Math|Random|RandomInteger (Utilities|Array|Length _randomizedcolor))))
  (Variables|/Script/UMG.TextBlock|SetText (Variables|/Game/Widgets/Sub_widget/W_Order_Recipe.W_Order_Recipe_C|GetRecipeName _w_orderrecpe) _name)
  (Variables|/Script/UMG.Image|SetBrush (Variables|/Game/Widgets/Sub_widget/W_Order_Recipe.W_Order_Recipe_C|GetRecipeIcon _w_orderrecpe) (Class|WidgetBlueprintLibrary|MakeBrushfromTexture _recipeimage 50 50)))