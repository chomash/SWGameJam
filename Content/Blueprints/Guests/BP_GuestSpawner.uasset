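; Guest spawner actor that spawns one AI guest, picked at random from its GuestsList of pawn classes.
; On BeginPlay it casts the game mode to GM_Base, stores the reference and calls SpawnGuest, so nothing spawns if the cast fails.
; SpawnGuest uses SpawnAIFromClass at the spawner's own location and rotation.
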(event Custom|SpawnGuest
  (bind _returnvalue (Transformation|GetActorTransform))
  (bind _guestslist (Variables|Default|GetGuestsList))
  (AI|SpawnAIFromClass (Utilities|Array|Get(acopy) _guestslist (Math|Random|RandomIntegerinRange 0 (- (Utilities|Array|Length _guestslist) 1))) 0 (.location _returnvalue) (.rotation _returnvalue) false 0))

(event EventBeginPlay
  (bind _asgm_base (Utilities|Casting|CastToGM_Base (Game|GetGameMode)))
  (Variables|Default|SetGameMode _asgm_base)
  (CallFunction|SpawnGuest))

(event Collision|EventActorBeginOverlap
  (params (OtherActor :type Actor%20Object%20Reference)))

(event EventTick
  (params (DeltaSeconds :type Float%20%28single-precision%29)))

(fn ConstructionScript)