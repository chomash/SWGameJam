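; BP_Guest is a guest that walks in along set targets when it begins play and walks out when told to leave.
; On BeginPlay it plays a bell sound, registers itself as GM_Base's ActiveGuest and finds the BP_GuestSpawner.
; Chained AIMoveTo calls take it through the spawner's first two TargetList entries.
; GuestExit moves it through the next two, then destroys it on arrival.
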(event Custom|GuestExit
  (bind _self self)
  ;[1 1 1] Comment
  (AI|AIMoveTo _self "0, 0, 0" (Utilities|Array|Get(acopy) (Variables|/Game/Blueprints/Guests/BP_GuestSpawner.BP_GuestSpawner_C|GetTargetList (Variables|Default|GetSpawnerRef)) 2) 5.0 false
    (:OnSuccess
      (AI|AIMoveTo _self "0, 0, 0" (Utilities|Array|Get(acopy) (Variables|/Game/Blueprints/Guests/BP_GuestSpawner.BP_GuestSpawner_C|GetTargetList (Variables|Default|GetSpawnerRef)) 3) 5.0 false
        (:OnSuccess
          (Actor|DestroyActor))))))

(event EventBeginPlay
  (bind _self self)
  (Audio|PlaySoundatLocation "/Game/Sounds/bell_Cue.bell_Cue" (Transformation|GetActorLocation) "0, 0, 0" 1.0 1.0 0.0 0 0 0 0)
  (bind _asgm_base (Utilities|Casting|CastToGM_Base (Game|GetGameMode)))
  (Variables|/Game/Blueprints/GM_Base.GM_Base_C|SetActiveGuest _asgm_base self)
  (bind _returnvalue (Actor|GetActorOfClass "/Game/Blueprints/Guests/BP_GuestSpawner.BP_GuestSpawner_C"))
  (Variables|Default|SetSpawnerRef _returnvalue)
  (AI|AIMoveTo _self "0, 0, 0" (Utilities|Array|Get(acopy) (Variables|/Game/Blueprints/Guests/BP_GuestSpawner.BP_GuestSpawner_C|GetTargetList (Variables|Default|GetSpawnerRef))) 5.0 false
    (:OnSuccess
      (AI|AIMoveTo _self "0, 0, 0" (Utilities|Array|Get(acopy) (Variables|/Game/Blueprints/Guests/BP_GuestSpawner.BP_GuestSpawner_C|GetTargetList (Variables|Default|GetSpawnerRef)) 1) 5.0 false))))

(fn ConstructionScript)