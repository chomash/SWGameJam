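; Bongo is a smokable furniture prop that plays a sound and a timed post-process effect when DoIT fires.
; A sphere overlap with the player map character toggles CanInteract and the prompt widget's visibility.
; The BongoTime timeline curve scales a boosted Intensity, based on settings cached at BeginPlay, on the first PostProcessVolume found.
; JustSmoked blocks retriggering until the timeline finishes.
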(event OnComponentBeginOverlap(Sphere)
  (params (OverlappedComponent :type Primitive%20Component%20Object%20Reference) (OtherActor :type Actor%20Object%20Reference) (OtherComp :type Primitive%20Component%20Object%20Reference) (OtherBodyIndex :type Integer) (bFromSweep :type Boolean) (SweepResult :type Hit%20Result%20Structure%20%28by%20ref%29))
  (Utilities|Casting|CastToBP_PlayerMapCharacter OtherActor)
  (Variables|Default|SetCanInteract true)
  (Rendering|SetVisibility (Variables|Default|GetWidget) true false))

(event OnComponentEndOverlap(Sphere)
  (params (OverlappedComponent :type Primitive%20Component%20Object%20Reference) (OtherActor :type Actor%20Object%20Reference) (OtherComp :type Primitive%20Component%20Object%20Reference) (OtherBodyIndex :type Integer))
  (Utilities|Casting|CastToBP_PlayerMapCharacter OtherActor)
  (Variables|Default|SetCanInteract false)
  (Rendering|SetVisibility (Variables|Default|GetWidget) false false))

(event Custom|DoIT
  (if (not (Variables|Default|GetJustSmoked))
    (Variables|Default|SetJustSmoked true)
    (Components|Timeline|PlayfromStart (Variables|Default|GetBongoTime))
    (Audio|PlaySoundatLocation "/Game/Sounds/bongo_Cue.bongo_Cue" (Transformation|GetWorldLocation (Variables|Default|GetDefaultSceneRoot)) "0, 0, 0" 1.0 1.0 0.0 0 0 0 0)))

(event EventBeginPlay
  (bind _returnvalue (Actor|GetActorOfClass "/Script/Engine.PostProcessVolume"))
  (bind _output_get (Variables|Default|SetPostProces _returnvalue))
  (Variables|Default|SetPPSettings (Variables|/Script/Engine.PostProcessVolume|GetSettings _output_get)))

(fn ConstructionScript)