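; Trash bin furniture actor that destroys map items placed inside its box volume.
; Every Tick it polls the box for overlapping BP_MapItem actors, destroys each one and activates a burst particle system without resetting it.
; The box's begin and end overlap events show and hide a widget, with no filter on which actor overlaps.
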(event OnComponentBeginOverlap(Box)
  (params (OverlappedComponent :type Primitive%20Component%20Object%20Reference) (OtherActor :type Actor%20Object%20Reference) (OtherComp :type Primitive%20Component%20Object%20Reference) (OtherBodyIndex :type Integer) (bFromSweep :type Boolean) (SweepResult :type Hit%20Result%20Structure%20%28by%20ref%29))
  (Rendering|SetVisibility (Variables|Default|GetWidget) true false))

(event OnComponentEndOverlap(Box)
  (params (OverlappedComponent :type Primitive%20Component%20Object%20Reference) (OtherActor :type Actor%20Object%20Reference) (OtherComp :type Primitive%20Component%20Object%20Reference) (OtherBodyIndex :type Integer))
  (Rendering|SetVisibility (Variables|Default|GetWidget) false false))

(event EventBeginPlay)

(event Collision|EventActorBeginOverlap
  (params (OtherActor :type Actor%20Object%20Reference)))

(event EventTick
  (params (DeltaSeconds :type Float%20%28single-precision%29))
  (bind _array_element (Utilities|Array|ForEachLoopwithBreak (Collision|GetOverlappingActors (Variables|Default|GetBox) "/Game/Blueprints/PickUps/BP_MapItem.BP_MapItem_C" :!class /Script/Engine.PrimitiveComponent))
    (:LoopBody
      (Variables|Default|SetItemToDestroy _array_element)
      (Actor|DestroyActor (Variables|Default|GetItemToDestroy))
      (Components|Activation|Activate (Variables|Default|GetP_Burst_System) false))))

(fn ConstructionScript)