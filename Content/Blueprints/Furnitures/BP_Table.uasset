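; BP_Table is a furniture actor that holds pickable map items in four slots.
; While a free-socket flag is set, Tick scans overlapping "MapPickable" actors for BP_MapItems neither held nor on a table.
; Each found item takes the first empty ItemsOnTable index, snaps to the matching scene component, and records its slot and on-table state.
; The free-socket flag is read but never updated in this graph.
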(event EventBeginPlay
  (Variables|Default|SetSockets "NewEnumerator0"))

(event EventTick
  (params (DeltaSeconds :type Float%20%28single-precision%29))
  (bind _itemsontable (Variables|Default|GetItemsOnTable))
  (if (Variables|Default|GetIsAnySocketFree)
    (bind _array_element (Utilities|Array|ForEachLoopwithBreak (Collision|GetOverlappingActors 0 :!class /Script/Engine.Actor))
      (:LoopBody
        (if (Actor|ActorHasTag _array_element "MapPickable")
          (bind _asbp_map_item (Utilities|Casting|CastToBP_MapItem _array_element))
          (Variables|Default|SetHeldItem _asbp_map_item)
          (if (not (Variables|/Game/Blueprints/PickUps/BP_MapItem.BP_MapItem_C|GetIsHeld _asbp_map_item))
            (if (not (Variables|/Game/Blueprints/PickUps/BP_MapItem.BP_MapItem_C|GetIsOnTable _asbp_map_item))
              (bind (_array_element_2 _array_index) (Utilities|Array|ForEachLoopwithBreak _itemsontable :!label _label)
                (:LoopBody
                  (Utilities|IsValid _array_element_2
                    (:Is%20Not%20Valid
                      (Variables|Default|SetAddItemHere _array_index)
                      (goto _label Break))))
                (:Completed
                  (Utilities|IsValid (Utilities|Array|Get(acopy) _itemsontable (Variables|Default|GetAddItemHere))
                    (:Is%20Not%20Valid
                      (Utilities|Array|SetArrayElem (Variables|Default|GetItemsOnTable) (Variables|Default|GetAddItemHere) (Variables|Default|GetHeldItem))
                      (switch int (Variables|Default|GetAddItemHere)
                        (:0
                          (Transformation|AttachComponentToComponent (Variables|Default|GetHeldItem) (Variables|Default|GetScene) "" "SnapToTarget" "SnapToTarget" "KeepWorld" true)
                          (Variables|/Game/Blueprints/PickUps/BP_MapItem.BP_MapItem_C|SetIsOnTable (Variables|Default|GetHeldItem) true)
                          (Variables|/Game/Blueprints/PickUps/BP_MapItem.BP_MapItem_C|SetItemSlot (Variables|Default|GetHeldItem) 0)
                          (Development|PrintString "one set"))
                        (:1
                          (Transformation|AttachComponentToComponent (Variables|Default|GetHeldItem) (Variables|Default|GetScene1) "" "SnapToTarget" "SnapToTarget" "KeepWorld" true)
                          (Variables|/Game/Blueprints/PickUps/BP_MapItem.BP_MapItem_C|SetIsOnTable (Variables|Default|GetHeldItem) true)
                          (Variables|/Game/Blueprints/PickUps/BP_MapItem.BP_MapItem_C|SetItemSlot (Variables|Default|GetHeldItem) 1)
                          (Development|PrintString "two set"))
                        (:2
                          (Transformation|AttachComponentToComponent (Variables|Default|GetHeldItem) (Variables|Default|GetScene2) "" "SnapToTarget" "SnapToTarget" "KeepWorld" true)
                          (Variables|/Game/Blueprints/PickUps/BP_MapItem.BP_MapItem_C|SetIsOnTable (Variables|Default|GetHeldItem) true)
                          (Variables|/Game/Blueprints/PickUps/BP_MapItem.BP_MapItem_C|SetItemSlot (Variables|Default|GetHeldItem) 2)
                          (Development|PrintString "three set"))
                        (:3
                          (Transformation|AttachComponentToComponent (Variables|Default|GetHeldItem) (Variables|Default|GetScene3) "" "SnapToTarget" "SnapToTarget" "KeepWorld" true)
                          (Variables|/Game/Blueprints/PickUps/BP_MapItem.BP_MapItem_C|SetIsOnTable (Variables|Default|GetHeldItem) true)
                          (Variables|/Game/Blueprints/PickUps/BP_MapItem.BP_MapItem_C|SetItemSlot (Variables|Default|GetHeldItem) 3)
                          (Development|PrintString "four set"))))))))))))))

(fn ConstructionScript)