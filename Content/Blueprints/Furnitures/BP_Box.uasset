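; BP_Box is a furniture Blueprint that acts as a dispenser, restocking itself with a configurable item class.
; Tick checks a flag and, when the box is empty, spawns the item at the Scene component's transform, attaches it there and stores its reference.
; When that item stops overlapping the box, a one-second delay clears the flag so a replacement spawns.
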(event EventBeginPlay)

(event Collision|EventActorBeginOverlap
  (params (OtherActor :type Actor%20Object%20Reference)))

(event EventTick
  (params (DeltaSeconds :type Float%20%28single-precision%29))
  (if (not (Variables|Default|GetIsItemOnBox))
    (bind _returnvalue (Class|MovieSceneTransformOrigin|GetTransformOrigin(Message) (Variables|Default|GetScene)))
    (bind _returnvalue_2 (Game|SpawnActorfromClass (Variables|Default|GetSpawnableItem) _returnvalue "Undefined" "MultiplyWithRoot" 0 0))
    (Variables|Default|SetNewlySpawnedItem _returnvalue_2)
    (Transformation|AttachComponentToComponent _returnvalue_2 (Variables|Default|GetScene) "None" "KeepRelative" "KeepRelative" "KeepRelative" true)
    (Variables|Default|SetIsItemOnBox true)))

(event Collision|EventActorEndOverlap
  (params (OtherActor :type Actor%20Object%20Reference))
  (if (== OtherActor (Variables|Default|GetNewlySpawnedItem))
    (Utilities|FlowControl|Delay 1.0)
    (Variables|Default|SetIsItemOnBox false)))

(fn ConstructionScript)