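; BP_Delliver is a furniture actor that acts as a drop spot, snapping potion items into place.
; While empty, it polls its Box every Tick for overlapping BP_MapItem actors tagged MapPotion.
; A match is stored as HeldItem, attached to the Scene component, and sets IsItemOnBox to stop further checks.
; Any actor end-overlap clears that flag after a one-second delay, leaving HeldItem set.
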(event EventBeginPlay)

(event Collision|EventActorBeginOverlap
  (params (OtherActor :type Actor%20Object%20Reference)))

(event EventTick
  (params (DeltaSeconds :type Float%20%28single-precision%29))
  (if (not (Variables|Default|GetIsItemOnBox))
    (bind _array_element (Utilities|Array|ForEachLoopwithBreak (Collision|GetOverlappingActors (Variables|Default|GetBox) "/Game/Blueprints/PickUps/BP_MapItem.BP_MapItem_C" :!class /Script/Engine.PrimitiveComponent))
      (:LoopBody
        (if (Actor|ActorHasTag _array_element "MapPotion")
          (bind _asbp_map_item (Utilities|Casting|CastToBP_MapItem _array_element))
          (Variables|Default|SetHeldItem _asbp_map_item)
          (Transformation|AttachComponentToComponent (Variables|Default|GetHeldItem) (Variables|Default|GetScene) "None" "SnapToTarget" "SnapToTarget" "KeepWorld" true)
          (Variables|Default|SetIsItemOnBox true))))))

(event Collision|EventActorEndOverlap
  (params (OtherActor :type Actor%20Object%20Reference))
  (Utilities|FlowControl|Delay 1.0)
  (Variables|Default|SetIsItemOnBox false))

(fn ConstructionScript)